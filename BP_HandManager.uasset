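; Hand manager actor that holds the player's deck of card row names and the 3D cards in hand.
; DrawCard takes the top deck entry, reads DT_UnitData, and spawns an attached BP_Card with that data.
; Drawing and hover changes run UpdateHandLayout, which gives cards target transforms in a centered fan with depth stagger and parabolic drop.
; Selected cards are left out of the spacing, and cards either side of the hovered one spread apart.
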(event `DrawCard`
  ; 抽卡
  ;; 判断卡组里是否有牌
  (if (> (`KismetArrayLibrary.Array_Length` (`self.DeckCards`)) 0)
    ;; 拿出卡组数组中的第 0 项，把这个名字传给GetDataTableRow，去DT_UnitData 数据表中检索
    (bind _returnvalue (`|GetDataTableRow` "/Game/DT/DT_UnitData.DT_UnitData" (`|GetArrayItem` (`self.DeckCards`)))
      (:`then`
        ;; 把最上面那张牌从清单里抹掉，原来的第 1 张变成了新的第 0 张
        (`KismetArrayLibrary.Array_Remove` (`self.DeckCards`))
        ;; 命令引擎生成一个BP_Card的实体
        (bind _returnvalue_2 (`|SpawnActorFromClass` "/Game/BP/BP_Card.BP_Card_C" (`self.GetTransform`) "Undefined" "MultiplyWithRoot" null null))
        (set `/Game/BP/BP_Card.CardInfo` _returnvalue _returnvalue_2)
        ;; 把3D卡牌，Add 到HandCards里
        (`KismetArrayLibrary.Array_Add` (`self.HandCards`) _returnvalue_2)
        ;; 把这张3D卡牌附加到管理器的DefaultSceneRoot上
        (`self.K2_AttachToComponent` _returnvalue_2 (`self.DefaultSceneRoot`) "None" "SnapToTarget" "SnapToTarget" "KeepRelative" true)
        (`self.UpdateHandLayout`)
        (`/Game/BP/BP_Card.SetCardStats` _returnvalue_2)))
    (else
      (`KismetSystemLibrary.PrintString` "没有卡！"))))

(event `SetHoverCard`
  (params (Card :type "/Game/BP/BP_Card Object Reference"))
  ; 鼠标正悬停在哪张卡上
  (set `self.HoveredCard` Card)
  (`self.UpdateHandLayout`))

(event `ClearHoverCard`
  (params (Card :type "/Game/BP/BP_Card Object Reference"))
  ; 当鼠标离开卡牌时，取消它的悬停状态
  (if (== (`self.HoveredCard`) Card)
    (set `self.HoveredCard` null)
    (`self.UpdateHandLayout`)))

(event `AddCardToDeck`
  (params (CardRowName :type Name))
  ; 将一个新获得的卡牌代号，塞进卡组清单里
  (if (< (`KismetArrayLibrary.Array_Length` (`self.DeckCards`)) (`self.MaxDeckSize`))
    (`KismetArrayLibrary.Array_Add` (`self.DeckCards`) CardRowName)
    (else
      (`KismetSystemLibrary.PrintString` "卡组已满"))))

(event `RemoveCardFromDeck`
  (params (CardRowNam :type Name))
  ; 精确撕毁/丢弃卡组里的某一张牌
  (`KismetArrayLibrary.Array_RemoveItem` (`self.DeckCards`) CardRowNam))

(fn `UpdateHandLayout`
  (locals (StartOffset :type "Float (double-precision)") (`Array Index` :type Integer) (SpreadOffset :type "Float (double-precision)") (HoverIndex :type Integer :default 0) (ActiveCount :type Integer) (VisualIndex :type Integer))
  (bind _visualindex (`local.VisualIndex`))
  (bind _returnvalue (- (`KismetMathLibrary.Conv_IntToDouble` (`local.VisualIndex`)) (/ (- (`KismetMathLibrary.Conv_IntToDouble` (`local.ActiveCount`)) 1.0) 2.0)))
  ; 排版开始前将有效手牌数量归零
  (set `local.ActiveCount` 0)
  ; 遍历所有手牌并判断是否有被鼠标抓起
  (for _array_element (`self.HandCards`)
    (if (not (`/Game/BP/BP_Card.IsSelected` _array_element))
      ; 如果没有被抓起，则有效手牌数+1
      (bind _output_get (set `local.ActiveCount` (+ (`local.ActiveCount`) 1)))))
  ; 计算最左边第一张卡牌应该放在哪个 Y 轴坐标上，把结果赋予StartOffset
  (set `local.StartOffset` (/ (* (- _output_get 1) (`self.CardSpacing`)) -2.0))
  ; 将VisualIndex归零，并检查手牌中的卡牌是否被拾起
  (set `local.VisualIndex` 0)
  (for (_array_element_2 _array_index) (`self.HandCards`)
    ; 扇形倾斜角度
    (set `/Game/BP/BP_Card.TargetRotation` (`KismetMathLibrary.MakeRotator` (* _returnvalue (`self.FanAngle`))) _array_element_2)
    (if (not (`/Game/BP/BP_Card.IsSelected` _array_element_2))
      (set `local.Array Index` _array_index)
      ; 判断当前处理的这张牌，在不在被悬停的牌的旁边，并决定它要让出多少距离
      (bind _output_get_2 (set `local.HoverIndex` (`KismetArrayLibrary.Array_Find` (`self.HandCards`) (`self.HoveredCard`))))
      (if (== _output_get_2 -1)
        (set `local.SpreadOffset` 0.0)
        ; 把前面算出的所有偏移量组合起来，告诉每张卡牌应该在什么位置
        (set `/Game/BP/BP_Card.TargetLocation` (`KismetMathLibrary.MakeVector` (* _visualindex (`self.DepthSpacing`)) (+ (+ (* _visualindex (`self.CardSpacing`)) (`local.StartOffset`)) (`local.SpreadOffset`)) (* (* (`self.FanHeightDrop`) -1.0) (* _returnvalue _returnvalue))) _array_element_2 :!label _label)
        ; 只有当一张牌真正被摆到了桌面上时，这个序号才会加 1
        (set `local.VisualIndex` (+ (`local.VisualIndex`) 1))
        (elif (< (`local.Array Index`) (`local.HoverIndex`))
          (set `local.SpreadOffset` (* (`self.SpreadDistance`) -1.0))
          (goto _label)
          (elif (> (`local.Array Index`) (`local.HoverIndex`))
            (set `local.SpreadOffset` (`self.SpreadDistance`))
            (goto _label)
            (elif (== (`local.Array Index`) (`local.HoverIndex`))
              (set `local.SpreadOffset` 0.0)
              (goto _label))))))))

(fn `UserConstructionScript`)