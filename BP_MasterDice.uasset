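; BP_MasterDice is a physics dice actor that reports its roll to BP_Controller for advantage/disadvantage resolution.
; A looping timer waits until velocity is low, then reads top and bottom faces from socket heights and DiceValues, sending the top.
; It spawns clone dice in an orbiting ring, later released with random velocities and their own result checks.
; A timeline handles spread movement, and hard impacts play a sound when not dragging.
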(event `CheckIsStopped`
  ; 检测骰子是否停下
  (if (< (`KismetMathLibrary.VSize` (`self.GetVelocity`)) 10.0)
    ;; 关闭计时器
    (`KismetSystemLibrary.K2_ClearAndInvalidateTimerHandle` (stale `StartResultCheck` _returnvalue))
    ;; 调用函数
    (`self.CalculateResult`)
    (bind _asbp_controller (cast `/Game/BP/BP_Controller` (`GameplayStatics.GetPlayerController` 0)))
    (`/Game/BP/BP_Controller.ADVorDISResult` _asbp_controller (`self.HighestPoint`))))

(event `StartResultCheck`
  ; 检测骰子是否停下
  (`KismetSystemLibrary.Delay` 0.5)
  (bind _returnvalue (`KismetSystemLibrary.K2_SetTimerDelegate` (delegate `CheckIsStopped`) 0.2 true)))

(event `PlaySpreadAnimation`
  (params (TargetPos :type "Vector Structure"))
  ; 6枚骰子在0.1秒扩散位移
  (set `self.IsSpreading` true)
  (`PrimitiveComponent.SetSimulatePhysics` (`self.DiceMesh`) false)
  (set `self.AnimStartPos` (`self.K2_GetActorLocation`))
  (bind (_direction _alpha) (`Timeline|SpreadTimeline` :!via `PlayFromStart`)
    (:`Update`
      (`SceneComponent.K2_SetWorldLocation` (`self.DiceMesh`) (`KismetMathLibrary.VLerp` (`self.AnimStartPos`) TargetPos _alpha) false false))
    (:`Finished`
      (set `self.IsSpreading` false))))

(event `SpawnClones`
  (params (CloneCount :type Integer) (ClassToSpawn :type "/BP_MasterDice Class Reference"))
  ; 生成克隆
  (if (> CloneCount 0)
    (for _index (range 1 (+ CloneCount 1))
      (bind _returnvalue (`|SpawnActorFromClass` ClassToSpawn (`KismetMathLibrary.Conv_VectorToTransform` (+ (`self.K2_GetActorLocation`) (* (`KismetMathLibrary.GetForwardVector` (`KismetMathLibrary.MakeRotator` 0.0 0.0 (`KismetMathLibrary.Conv_IntToDouble` (* _index (/ 360 CloneCount))))) 500.0))) "AlwaysSpawn" "MultiplyWithRoot" null null null))
      (`KismetArrayLibrary.Array_Add` (`self.AttachedClones`) _returnvalue)
      (`self.SetActorEnableCollision` _returnvalue false)
      (`PrimitiveComponent.SetSimulatePhysics` (`/BP_MasterDice.DiceMesh` _returnvalue) false)
      (`self.K2_AttachToComponent` _returnvalue (`self.OrbitCenter`) "None" "KeepWorld" "KeepWorld" "KeepWorld" true))))

(event `Destroyed`
  ; 右键销毁克隆体
  (for _array_element (`self.AttachedClones`)
    (`self.K2_DestroyActor` _array_element)))

(event `ReleaseClones`
  (bind _returnvalue (`KismetMathLibrary.RandomFloatInRange` -500.0 500.0))
  ; 投出克隆骰
  (for _array_element (`self.AttachedClones`)
    (`self.K2_DetachFromActor` _array_element "KeepWorld" "KeepWorld" "KeepWorld")
    (`self.SetActorEnableCollision` _array_element true)
    (bind _dicemesh (`/BP_MasterDice.DiceMesh` _array_element))
    (`PrimitiveComponent.SetSimulatePhysics` _dicemesh true)
    (bind _returnvalue_2 (`PrimitiveComponent.GetPhysicsLinearVelocity` _dicemesh "None"))
    (`PrimitiveComponent.SetPhysicsLinearVelocity` _dicemesh (+ _returnvalue_2 (* (`KismetMathLibrary.RandomUnitVector`) 300.0)) false "None")
    (`PrimitiveComponent.SetPhysicsAngularVelocityInDegrees` _dicemesh (`KismetMathLibrary.MakeVector` _returnvalue _returnvalue _returnvalue) false "None")
    (`self.StartResultCheck` _array_element))
  (`KismetArrayLibrary.Array_Clear` (`self.AttachedClones`)))

(event `self.ReceiveTick`
  (params (DeltaSeconds :type "Float (single-precision)"))
  ; 克隆骰旋转
  (if (> (`KismetArrayLibrary.Array_Length` (`self.AttachedClones`)) 0)
    (`SceneComponent.K2_AddWorldRotation` (`self.OrbitCenter`) (`KismetMathLibrary.MakeRotator` 0.0 0.0 (* DeltaSeconds (* (`self.OrbitSpeed`) (`KismetMathLibrary.SelectFloat` 1.0 -1.0 (`self.OrbitClockwise`))))) false false)))

(event `OnDiceImpact`
  ; 碰撞发声
  (bind _asbp_controller (cast `/Game/BP/BP_Controller` (`GameplayStatics.GetPlayerController` 0)))
  (if (`/Game/BP/BP_Controller.IsDiceDragging` _asbp_controller)
    _
    (elif (> (`KismetMathLibrary.VSize` (`self.GetVelocity`)) 300.0)
      (`GameplayStatics.PlaySoundAtLocation` "/Engine/EngineSounds/1kSineTonePing.1kSineTonePing" (`self.K2_GetActorLocation`) (struct) 1.0 1.0 0.0 null null null null))))

(event `self.DiceMesh.OnBeginCursorOver`
  (params (TouchedComponent :type "PrimitiveComponent Object Reference")))

(event `self.DiceMesh.OnEndCursorOver`
  (params (TouchedComponent :type "PrimitiveComponent Object Reference")))

(event `self.ReceiveHit`
  (params (MyComp :type "PrimitiveComponent Object Reference") (Other :type "Actor Object Reference") (OtherComp :type "PrimitiveComponent Object Reference") (bSelfMoved :type Boolean) (HitLocation :type "Vector Structure") (HitNormal :type "Vector Structure") (NormalImpulse :type "Vector Structure") (Hit :type "HitResult Structure (by ref)"))
  (`self.OnDiceImpact`))

(fn `CalculateResult`
  (locals (HighestZ :type "Float (double-precision)" :default -9999.0) (TopSocket :type String) (LowestZ :type "Float (double-precision)" :default 9999.0) (BottomSocket :type String))
  (bind _value (`BlueprintMapLibrary.Map_Find` (`self.DiceValues`) (`local.TopSocket`)))
  ; 遍历骰子的所有面
  (for _array_element (`SceneComponent.GetAllSocketNames` (`self.DiceMesh`))
    (`|ExecutionSequence`
      (:`then_0`
        (bind (_returnvalue_x _returnvalue_y _returnvalue_z) (`KismetMathLibrary.BreakVector` (`SceneComponent.GetSocketLocation` (`self.DiceMesh`) _array_element)))
        ; 如果发现了更高的面，则设置HighestZ=当前的 Z，TopSocket=Socket
        (if (> _returnvalue_z (`local.HighestZ`))
          (set `local.HighestZ` _returnvalue_z)
          (set `local.TopSocket` (`KismetStringLibrary.Conv_NameToString` _array_element))))
      (:`then_1`
        ; 找到最低面
        (if (< _returnvalue_z (`local.LowestZ`))
          (set `local.LowestZ` _returnvalue_z)
          (set `local.BottomSocket` (`KismetStringLibrary.Conv_NameToString` _array_element))))))
  (set `self.HighestPoint` _value)
  (set `self.LowestPoint` (`BlueprintMapLibrary.Map_Find` (`self.DiceValues`) (`local.BottomSocket`)))
  (`KismetSystemLibrary.PrintString` (`KismetStringLibrary.Conv_IntToString` _value)))

(fn `UserConstructionScript`)